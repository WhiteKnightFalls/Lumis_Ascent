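; BP_Ice is an ice zone that makes BP_TPCharacter slippery while inside its trigger.
; Entering Trigger_0 sets the character's ground friction and walking braking deceleration to the ice values.
; Leaving writes back this Blueprint's default variables rather than values saved from the character.
; Nodes setting max walk speed and acceleration are left unconnected and never run.
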(event `self.Trigger_0.OnComponentBeginOverlap`
  (params (OverlappedComponent :type "PrimitiveComponent Object Reference") (OtherActor :type "Actor Object Reference") (OtherComp :type "PrimitiveComponent Object Reference") (OtherBodyIndex :type Integer) (bFromSweep :type Boolean) (SweepResult :type "HitResult Structure (by ref)"))
  (bind _asbp_tpcharacter (cast `/Game/Blueprints/BP_TPCharacter` OtherActor))
  (bind _charactermovement (`Character.CharacterMovement` _asbp_tpcharacter))
  (set `CharacterMovementComponent.GroundFriction` (`self.IceGroundFriction`) _charactermovement)
  (set `CharacterMovementComponent.BrakingDecelerationWalking` (`self.IceBrakingDecceleration`) _charactermovement))

(event `self.Trigger_0.OnComponentEndOverlap`
  (params (OverlappedComponent :type "PrimitiveComponent Object Reference") (OtherActor :type "Actor Object Reference") (OtherComp :type "PrimitiveComponent Object Reference") (OtherBodyIndex :type Integer))
  (bind _asbp_tpcharacter (cast `/Game/Blueprints/BP_TPCharacter` OtherActor))
  (bind _charactermovement (`Character.CharacterMovement` _asbp_tpcharacter))
  (set `CharacterMovementComponent.GroundFriction` (`self.DefaultGroundFriction`) _charactermovement)
  (set `CharacterMovementComponent.BrakingDecelerationWalking` (`self.DefaultBrakingDecceleration`) _charactermovement))

(fn `UserConstructionScript`)