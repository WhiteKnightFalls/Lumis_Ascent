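; Player controller for the third-person character, turning Enhanced Input actions into calls on the possessed BP_TPCharacter.
; On possess it caches the character and adds the IMC_ThirdPerson mapping context, then forwards camera, move, interact and sprint input.
; Jump fires once per press through a DoOnce reset on release, toggling the character's gravity scale setting alongside it.
; Pause toggles a newly created BWP_PauseMenu widget together with game pause, input mode and mouse cursor.
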(event `self.ReceivePossess`
  (params (PossessedPawn :type "Pawn Object Reference"))
  (bind _asbp_tpcharacter (cast `/Game/Blueprints/BP_TPCharacter` PossessedPawn))
  (set `self.PossessedTPC` _asbp_tpcharacter)
  (`EnhancedInputSubsystemInterface.AddMappingContext` (subsystem `EnhancedInputLocalPlayerSubsystem`) "/Game/Input/IMC_ThirdPerson.IMC_ThirdPerson" 0 (struct)))

(event `EnhancedInput|/Game/Input/InputActions/IA_RotateCamera`
  (params (ActionValue :type "Vector2D Structure") (ElapsedSeconds :type "Float (double-precision)") (TriggeredSeconds :type "Float (double-precision)") (InputAction :type "InputAction Object Reference" :default "/Game/Input/InputActions/IA_RotateCamera.IA_RotateCamera"))
  (bind _possessedtpc (`self.PossessedTPC`))
  (:`Triggered`
    (`Pawn.AddControllerYawInput` _possessedtpc ActionValue_X)
    (`Pawn.AddControllerPitchInput` _possessedtpc ActionValue_Y)))

(event `EnhancedInput|/Game/Input/InputActions/IA_Jump`
  (params (ActionValue :type Boolean) (ElapsedSeconds :type "Float (double-precision)") (TriggeredSeconds :type "Float (double-precision)") (InputAction :type "InputAction Object Reference" :default "/Game/Input/InputActions/IA_Jump.IA_Jump"))
  (bind _possessedtpc (`self.PossessedTPC`))
  (:`Triggered`
    (if (`Character.CanJump` _possessedtpc)
      (`/Engine/EditorBlueprintResources/StandardMacros.DoOnce` false :!label _label
        (:`Completed`
          (`Character.Jump` _possessedtpc)
          (`/Game/Blueprints/BP_TPCharacter.SetGravityScale` _possessedtpc true)))))
  (:`Completed`
    (`/Game/Blueprints/BP_TPCharacter.SetGravityScale` (`self.PossessedTPC`) false)
    (goto _label :!via `Reset`)))

(event `EnhancedInput|/Game/Input/InputActions/IA_Move`
  (params (ActionValue :type "Vector2D Structure") (ElapsedSeconds :type "Float (double-precision)") (TriggeredSeconds :type "Float (double-precision)") (InputAction :type "InputAction Object Reference" :default "/Game/Input/InputActions/IA_Move.IA_Move"))
  (:`Triggered`
    (`/Game/Blueprints/BP_TPCharacter.MoveInWorldDirection` (`self.PossessedTPC`) (`KismetMathLibrary.MakeVector` ActionValue_X ActionValue_Y))))

(event `EnhancedInput|/Game/Input/InputActions/IA_Interact`
  (params (ActionValue :type Boolean) (ElapsedSeconds :type "Float (double-precision)") (TriggeredSeconds :type "Float (double-precision)") (InputAction :type "InputAction Object Reference" :default "/Game/Input/InputActions/IA_Interact.IA_Interact"))
  (:`Triggered`
    (`/Game/Blueprints/BP_TPCharacter.StartInteract` (`self.PossessedTPC`))))

(event `EnhancedInput|/Game/Input/InputActions/IA_Sprint`
  (params (ActionValue :type Boolean) (ElapsedSeconds :type "Float (double-precision)") (TriggeredSeconds :type "Float (double-precision)") (InputAction :type "InputAction Object Reference" :default "/Game/Input/InputActions/IA_Sprint.IA_Sprint"))
  (:`Triggered`
    (`KismetSystemLibrary.PrintString` "sprinting")
    (`/Game/Blueprints/BP_TPCharacter.Sprint` (`self.PossessedTPC`) true))
  (:`Completed`
    (`/Game/Blueprints/BP_TPCharacter.Sprint` (`self.PossessedTPC`) false)))

(event `EnhancedInput|/Game/Input/InputActions/IA_Pause`
  (params (ActionValue :type Boolean) (ElapsedSeconds :type "Float (double-precision)") (TriggeredSeconds :type "Float (double-precision)") (InputAction :type "InputAction Object Reference" :default "/Game/Input/InputActions/IA_Pause.IA_Pause"))
  (bind _returnvalue (`GameplayStatics.GetPlayerController` 0))
  (:`Started`
    (if (not (`self.isPauseMenuOpen`))
      (set `self.isPauseMenuOpen` true)
      (bind _returnvalue_2 (`|CreateWidget` "/Game/UI/BWP_PauseMenu.BWP_PauseMenu_C" _returnvalue))
      (bind _output_get (set `self.PausemenuWidget` _returnvalue_2))
      (`UserWidget.AddToViewport` _output_get 0)
      (`WidgetBlueprintLibrary.SetInputMode_GameAndUIEx` _returnvalue (`self.PausemenuWidget`))
      (set `PlayerController.bShowMouseCursor` true (`GameplayStatics.GetPlayerController` 0))
      (`GameplayStatics.SetGamePaused` true)
      (else
        (set `self.isPauseMenuOpen` false)
        (`Widget.RemoveFromParent` (`self.PausemenuWidget`))
        (`GameplayStatics.SetGamePaused` false)
        (`WidgetBlueprintLibrary.SetInputMode_GameOnly` _returnvalue)
        (set `PlayerController.bShowMouseCursor` false (`GameplayStatics.GetPlayerController` 0))))))

(fn `UserConstructionScript`)