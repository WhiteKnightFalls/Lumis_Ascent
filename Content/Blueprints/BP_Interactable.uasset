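; BP_Interactable is an interactable actor that shows a widget based on the player character's proximity.
; Overlap events on Collider and BoxCollider each set a flag for BP_TPCharacter, then call NewFunction to refresh visibility.
; The widget is visible only while the character overlaps Collider but not BoxCollider.
; The Interact event only prints a message.
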(event `Interact`
  (`KismetSystemLibrary.PrintString` "Interacted"))

(event `self.Collider.OnComponentBeginOverlap`
  (params (OverlappedComponent :type "PrimitiveComponent Object Reference") (OtherActor :type "Actor Object Reference") (OtherComp :type "PrimitiveComponent Object Reference") (OtherBodyIndex :type Integer) (bFromSweep :type Boolean) (SweepResult :type "HitResult Structure (by ref)"))
  (cast `/Game/Blueprints/BP_TPCharacter` OtherActor)
  (set `self.isOverlappingWithBox` true)
  (`self.NewFunction` :!label _label))

(event `self.Collider.OnComponentEndOverlap`
  (params (OverlappedComponent :type "PrimitiveComponent Object Reference") (OtherActor :type "Actor Object Reference") (OtherComp :type "PrimitiveComponent Object Reference") (OtherBodyIndex :type Integer))
  (cast `/Game/Blueprints/BP_TPCharacter` OtherActor)
  (set `self.isOverlappingWithBox` false)
  (goto _label))

(event `self.BoxCollider.OnComponentBeginOverlap`
  (params (OverlappedComponent :type "PrimitiveComponent Object Reference") (OtherActor :type "Actor Object Reference") (OtherComp :type "PrimitiveComponent Object Reference") (OtherBodyIndex :type Integer) (bFromSweep :type Boolean) (SweepResult :type "HitResult Structure (by ref)"))
  (cast `/Game/Blueprints/BP_TPCharacter` OtherActor)
  (set `self.isOerlappingWithBox1` true)
  (goto _label))

(event `self.BoxCollider.OnComponentEndOverlap`
  (params (OverlappedComponent :type "PrimitiveComponent Object Reference") (OtherActor :type "Actor Object Reference") (OtherComp :type "PrimitiveComponent Object Reference") (OtherBodyIndex :type Integer))
  (cast `/Game/Blueprints/BP_TPCharacter` OtherActor)
  (set `self.isOerlappingWithBox1` false)
  (goto _label))

(fn `NewFunction`
  (`SceneComponent.SetVisibility` (`self.Widget`) (and (`self.isOverlappingWithBox`) (not (`self.isOerlappingWithBox1`))) false))

(fn `UserConstructionScript`)