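; Game instance that loads saved settings on startup, or creates a new save object, and writes it back to the Settings slot on shutdown.
; Init retries each tick until a game mode exists, then applies sound class overrides and pushes the sound mix.
; Master, music and SFX classes all take their volume from the saved MasterVolume.
; ReturnSettingsSave exposes the settings object to other code.
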(event `self.ReceiveInit`
  (bind _returnvalue (`GameplayStatics.DoesSaveGameExist` (`self.Settings`)))
  (if _returnvalue
    (bind _returnvalue_2 (`GameplayStatics.LoadGameFromSlot` (`self.Settings`)))
    (bind _asbp_save_game_settings_save (cast `/Game/Blueprints/BP_SaveGame_SettingsSave` _returnvalue_2))
    (set `self.SettingsSave` _asbp_save_game_settings_save)
    (else
      (bind _returnvalue_3 (`GameplayStatics.CreateSaveGameObject` "/Game/Blueprints/BP_SaveGame_SettingsSave.BP_SaveGame_SettingsSave_C"))
      (set `self.SettingsSave` _returnvalue_3)))
  (`/Engine/EditorBlueprintResources/StandardMacros.IsValid` (`GameplayStatics.GetGameMode`) :!label _label
    (:`Is Valid`
      (`GameplayStatics.SetSoundMixClassOverride` "/Game/Audio/SoundMixer/SoundMix.SoundMix" "/Game/Audio/SoundMixer/MixerMaster.MixerMaster" (`/Game/Blueprints/BP_SaveGame_SettingsSave.MasterVolume` (`self.SettingsSave`)) 1.0 0.0)
      (`GameplayStatics.SetSoundMixClassOverride` "/Game/Audio/SoundMixer/SoundMix.SoundMix" "/Game/Audio/SoundMixer/MixerMusic.MixerMusic" (`/Game/Blueprints/BP_SaveGame_SettingsSave.MasterVolume` (`self.SettingsSave`)) 1.0 0.0)
      (`GameplayStatics.SetSoundMixClassOverride` "/Game/Audio/SoundMixer/SoundMix.SoundMix" "/Game/Audio/SoundMixer/MixerSFX.MixerSFX" (`/Game/Blueprints/BP_SaveGame_SettingsSave.MasterVolume` (`self.SettingsSave`)) 1.0 0.0)
      (`GameplayStatics.PushSoundMixModifier` "/Game/Audio/SoundMixer/SoundMix.SoundMix"))
    (:`Is Not Valid`
      (`KismetSystemLibrary.DelayUntilNextTick`)
      (goto _label))))

(event `self.ReceiveShutdown`
  (`GameplayStatics.SaveGameToSlot` (`self.SettingsSave`) (`self.Settings`)))

(fn `ReturnSettingsSave`
  (returns (SettingsSaveRef :type "/Game/Blueprints/BP_SaveGame_SettingsSave Object Reference"))
  (return (`self.SettingsSave`)))