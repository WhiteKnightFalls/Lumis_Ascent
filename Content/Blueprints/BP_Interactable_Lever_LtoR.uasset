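; Lever interactable that starts a left-to-right moving platform and lights a rune rock when used.
; BeginPlay creates a dynamic material instance on the RuneRock for emission control.
; Interact calls the parent, then a DoOnce with no reset plays a sound, sets Emission to five minus its stored strength, and calls StartonInteractedLever on MovingPlatformLtoR, so the lever works only once.
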(event `self.ReceiveBeginPlay`
  (bind _returnvalue (`PrimitiveComponent.CreateDynamicMaterialInstance` (`self.RuneRock`) 0 null "None"))
  (set `self.MID` _returnvalue))

(event `self.Interact`
  (`parent.Interact`)
  (`/Engine/EditorBlueprintResources/StandardMacros.DoOnce` false
    (:`Completed`
      (`GameplayStatics.PlaySound2D` "/Game/Audio/SFX/SFX/Interactable.Interactable" 1.0 1.0 0.0 null null)
      (bind _output_get (set `self.EmissionSrength` (- 5.0 (`self.EmissionSrength`))))
      (`MaterialInstanceDynamic.SetScalarParameterValue` (`self.MID`) "Emission" _output_get)
      (`/Game/Blueprints/BP_InteractableLever_MovingPlatform.StartonInteractedLever` (`self.MovingPlatformLtoR`)))))

(fn `UserConstructionScript`
  (`parent.UserConstructionScript`))