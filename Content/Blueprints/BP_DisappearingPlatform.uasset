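; Platform Blueprint whose cube vanishes shortly after a BP_TPCharacter hits it.
; The Hit event swaps the cube to a red-only debug material, waits briefly, then hides it and disables its collision.
; The cube's end-overlap event waits the same delay, then restores material, visibility and collision.
; Two SetSimulatePhysics nodes are left unconnected and never run.
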(event `self.ReceiveHit`
  (params (MyComp :type "PrimitiveComponent Object Reference") (Other :type "Actor Object Reference") (OtherComp :type "PrimitiveComponent Object Reference") (bSelfMoved :type Boolean) (HitLocation :type "Vector Structure") (HitNormal :type "Vector Structure") (NormalImpulse :type "Vector Structure") (Hit :type "HitResult Structure (by ref)"))
  (cast `/Game/Blueprints/BP_TPCharacter` Other)
  (`PrimitiveComponent.SetMaterial` (`self.Cube`) 0 "/Engine/EngineDebugMaterials/VertexColorViewMode_RedOnly.VertexColorViewMode_RedOnly")
  (`KismetSystemLibrary.Delay` 2.0)
  (`SceneComponent.SetVisibility` (`self.Cube`) false false)
  (`PrimitiveComponent.SetCollisionEnabled` (`self.Cube`) "NoCollision"))

(event `self.Cube.OnComponentEndOverlap`
  (params (OverlappedComponent :type "PrimitiveComponent Object Reference") (OtherActor :type "Actor Object Reference") (OtherComp :type "PrimitiveComponent Object Reference") (OtherBodyIndex :type Integer))
  (`KismetSystemLibrary.Delay` 2.0)
  (`PrimitiveComponent.SetMaterial` (`self.Cube`) 0 "/Engine/EngineMaterials/CubeMaterial.CubeMaterial")
  (`SceneComponent.SetVisibility` (`self.Cube`) true false)
  (`PrimitiveComponent.SetCollisionEnabled` (`self.Cube`) "QueryAndPhysics"))

(fn `UserConstructionScript`)