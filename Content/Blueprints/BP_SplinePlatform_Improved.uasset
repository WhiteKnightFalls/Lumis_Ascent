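; Platform actor that travels continuously along the spline of an assigned spline actor, wrapping around at either end so it loops.
; Each tick it advances its distance by travel speed and delta time, then sets its world location and, optionally, its rotation from the spline.
; A start offset, as a fraction of spline length, places it in the construction script and at BeginPlay, which prints a warning if no spline is assigned.
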(event `self.ReceiveBeginPlay`
  (`parent.ReceiveBeginPlay`)
  ;[1 1 1] Set where platform should start
  (`/Engine/EditorBlueprintResources/StandardMacros.IsValid` (`self.SplineActor`)
    (:`Is Valid`
      (`self.Apply Start Offset`))
    (:`Is Not Valid`
      ;[1 0.2274 0.2274] Display warning if Spline actor is unassigned!
      (`KismetSystemLibrary.PrintString` "SplinePlatform: Spline actor is not assigned!" true true (struct :`R` 1.0 :`G` 0.053995 :`A` 1.0) 10.0))))

(event `self.ReceiveTick`
  (params (DeltaSeconds :type "Float (single-precision)"))
  (`parent.ReceiveTick` DeltaSeconds)
  ;[1 1 1] Move Platform along spline
  (`/Engine/EditorBlueprintResources/StandardMacros.IsValid` (`self.SplineActor`)
    (:`Is Valid`
      (`self.Update Distance Along Spline`)
      (`self.UpdateTransform`))))

(fn `Apply Start Offset`
  (set `self.Distance Along Spline` (* (`self.StartOffset`) (`SplineComponent.GetSplineLength` (`/Game/Blueprints/BP_SplineActor.Spline` (`self.SplineActor`))))))

(fn `ClampDistanceAlongSpline`
  (params (`Spline Length` :type "Float (single-precision)"))
  (`|ExecutionSequence`
    (:`then_0`
      ;[1 1 1] Make sure distance isnt overshot
      (if (>= (`self.Distance Along Spline`) (`local.Spline Length`))
        (set `self.Distance Along Spline` (- (`self.Distance Along Spline`) (`local.Spline Length`)))))
    (:`then_1`
      ;[1 1 1] Make sure distance cannot go below 0
      (if (< (`self.Distance Along Spline`) 0.0)
        (set `self.Distance Along Spline` (+ (`local.Spline Length`) (`self.Distance Along Spline`)))))))

(fn `Update Distance Along Spline`
  (set `self.Distance Along Spline` (+ (* (`GameplayStatics.GetWorldDeltaSeconds`) (`self.TravelSpeed`)) (`self.Distance Along Spline`)))
  (`self.ClampDistanceAlongSpline` (`SplineComponent.GetSplineLength` (`/Game/Blueprints/BP_SplineActor.Spline` (`self.SplineActor`)))))

(fn `UpdateLocation`
  (`self.K2_SetActorLocation` (`SplineComponent.GetLocationAtDistanceAlongSpline` (`/Game/Blueprints/BP_SplineActor.Spline` (`self.SplineActor`)) (`self.Distance Along Spline`) "World")))

(fn `UpdateRotation`
  (`self.K2_SetActorRotation` (`SplineComponent.GetRotationAtDistanceAlongSpline` (`/Game/Blueprints/BP_SplineActor.Spline` (`self.SplineActor`)) (`self.Distance Along Spline`) "World")))

(fn `UpdateTransform`
  (`self.UpdateLocation`)
  (if (`self.bAlignRotationToSpline`)
    (`self.UpdateRotation`)))

(fn `UserConstructionScript`
  (`/Engine/EditorBlueprintResources/StandardMacros.IsValid` (`self.SplineActor`)
    (:`Is Valid`
      (`self.Apply Start Offset`)
      (`self.UpdateTransform`))))