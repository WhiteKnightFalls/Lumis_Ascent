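; Interactable statue that toggles a glow on its mesh when the player interacts with it.
; On BeginPlay it creates a dynamic material instance on the Cube component.
; Interact calls the parent logic, then flips EmissionStrength by subtracting it from its maximum and writes it to the material parameter.
; IsOn derives the on/off state from that emission value rather than a separate boolean.
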(event `self.ReceiveBeginPlay`
  (bind _returnvalue (`PrimitiveComponent.CreateDynamicMaterialInstance` (`self.Cube`) 0 null "None"))
  (set `self.MID` _returnvalue))

(event `self.Interact`
  (`parent.Interact`)
  (bind _output_get (set `self.EmissionStrength` (- 10.0 (`self.EmissionStrength`))))
  (`MaterialInstanceDynamic.SetScalarParameterValue` (`self.MID`) "EmissionStrength" _output_get))

(fn `isOn`
  (returns (ReturnValue :type Boolean))
  (return (== (`self.EmissionStrength`) 10.0)))

(fn `UserConstructionScript`)