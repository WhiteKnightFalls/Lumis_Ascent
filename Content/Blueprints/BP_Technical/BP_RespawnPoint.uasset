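; BP_RespawnPoint is a checkpoint actor that sets itself as the respawn point of any overlapping BP_TPCharacter.
; Its Checkpoint component spins constantly on Tick.
; An overlap also plays a sound and a timeline-driven extra spin, gated by a DoOnce that resets when the timeline finishes.
; GetRespawnLocRot exposes the Pivot's world location and rotation as the respawn transform.
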(event `self.ReceiveTick`
  (params (DeltaSeconds :type "Float (single-precision)"))
  (`SceneComponent.K2_AddRelativeRotation` (`self.Checkpoint`) (`KismetMathLibrary.MakeRotator` 0.0 0.0 (* (`self.IdleRotSpeed`) (`GameplayStatics.GetWorldDeltaSeconds`))) false false))

(event `self.ReceiveActorBeginOverlap`
  (params (OtherActor :type "Actor Object Reference"))
  (bind _asbp_tpcharacter (cast `/Game/Blueprints/BP_Character/BP_TPCharacter` OtherActor))
  (set `/Game/Blueprints/BP_Character/BP_TPCharacter.MyRespawnPoint` self _asbp_tpcharacter)
  (`/Engine/EditorBlueprintResources/StandardMacros.DoOnce` false :!label _label
    (:`Completed`
      (`GameplayStatics.PlaySound2D` "/Game/Audio/SFX/SFX/Checkpoint.Checkpoint" 1.0 1.0 0.0 null null)
      (bind (_direction _newtrack_0) (`Timeline|Timeline` :!via `PlayFromStart`)
        (:`Update`
          (`SceneComponent.K2_AddRelativeRotation` (`self.Checkpoint`) (`KismetMathLibrary.MakeRotator` 0.0 0.0 (* _newtrack_0 (`self.relativeRotation`) (`GameplayStatics.GetWorldDeltaSeconds`))) false false)
          (`KismetSystemLibrary.Delay` 10.0))
        (:`Finished`
          (goto _label :!via `Reset`))))))

(fn `GetRespawnLocRot`
  (returns (Location :type "Vector Structure") (Rotation :type "Rotator Structure"))
  (return (`SceneComponent.K2_GetComponentLocation` (`self.Pivot`)) (`SceneComponent.K2_GetComponentRotation` (`self.Pivot`))))

(fn `UserConstructionScript`)