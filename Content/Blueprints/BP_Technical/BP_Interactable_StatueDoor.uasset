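; Interactable statue door that swings open or shut on alternate interactions while it is unlocked.
; A FlipFlop plays or reverses a timeline whose DoorOpen track rotates the Pivot up to 90 degrees in roll.
; A DoOnce, fed by IsLocked and reset when the timeline finishes, blocks further interactions while the door moves.
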(event `self.Interact`
  (`parent.Interact`)
  (`/Engine/EditorBlueprintResources/StandardMacros.DoOnce` (`self.isLocked`) :!label _label
    (:`Completed`
      (if (not (`self.isLocked`))
        (`/Engine/EditorBlueprintResources/StandardMacros.FlipFlop`
          (:`A`
            (bind (_direction _dooropen) (`Timeline|Timeline` :!label _label_2)
              (:`Update`
                (`SceneComponent.K2_SetRelativeRotation` (`self.Pivot`) (`KismetMathLibrary.MakeRotator` (* _dooropen 90.0)) false false))
              (:`Finished`
                (goto _label :!via `Reset`))))
          (:`B`
            (goto _label_2 :!via `Reverse`)))))))

(fn `UserConstructionScript`
  (`parent.UserConstructionScript`))