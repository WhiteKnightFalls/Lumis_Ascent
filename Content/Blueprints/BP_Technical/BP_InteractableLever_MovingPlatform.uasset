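; Moving platform that starts shuttling back and forth when its StartonInteractedLever event fires.
; After an initial delay, a FlipFlop alternately plays and reverses the Movement timeline, with a separate delay before each direction, looping on each finish.
; The timeline's MoveToPos output scales DirectionMovement to set the Cube's relative location without sweep.
; The node that sets play rate from TimeToComplete is never executed.
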(event `StartonInteractedLever`
  (`KismetSystemLibrary.Delay` (`self.DelayFirst`))
  (`/Engine/EditorBlueprintResources/StandardMacros.FlipFlop` :!label _label
    (:`A`
      (`KismetSystemLibrary.Delay` (`self.DelayEnd`))
      (bind (_direction _movetopos) (`Timeline|Movement` :!label _label_2)
        (:`Update`
          (`SceneComponent.K2_SetRelativeLocation` (`self.Cube`) (* _movetopos (`self.DirectionMovement`)) false false))
        (:`Finished`
          (goto _label))))
    (:`B`
      (`KismetSystemLibrary.Delay` (`self.DelayStart`))
      (goto _label_2 :!via `Reverse`))))

(fn `UserConstructionScript`)