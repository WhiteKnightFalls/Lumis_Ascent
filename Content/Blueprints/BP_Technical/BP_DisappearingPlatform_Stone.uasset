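; Stone platform that glows, shakes and disappears when a BP_TPCharacter steps into its trigger, then returns.
; Timelines drive the shake and opacity fade on a dynamic material, with visibility and collider collision switched off after a configurable delay.
; Trigger end-overlap waits, clears the glow, then fades the platform back in and restores collision.
; DoOnce gates limit retriggering; two vertical-movement timelines are present but unconnected.
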(event `self.ReceiveBeginPlay`
  (bind _returnvalue (`PrimitiveComponent.CreateDynamicMaterialInstance` (`self.Platform`) 0 "/Game/Assets/Platforms/Stone/MI_Platform_Stone_2.MI_Platform_Stone_2" "None"))
  (bind _output_get (set `self.DynamicMaterial` _returnvalue))
  (`MaterialInstanceDynamic.SetScalarParameterValue` _output_get "Emissive" 0.0))

(event `self.TriggerFade.OnComponentBeginOverlap`
  (params (OverlappedComponent :type "PrimitiveComponent Object Reference") (OtherActor :type "Actor Object Reference") (OtherComp :type "PrimitiveComponent Object Reference") (OtherBodyIndex :type Integer) (bFromSweep :type Boolean) (SweepResult :type "HitResult Structure (by ref)"))
  (cast `/Game/Blueprints/BP_Character/BP_TPCharacter` OtherActor)
  (`MaterialInstanceDynamic.SetScalarParameterValue` (`self.DynamicMaterial`) "Emissive" 1.0)
  (`|ExecutionSequence`
    (:`then_0`
      (`/Engine/EditorBlueprintResources/StandardMacros.DoOnce` false :!label _label
        (:`Completed`
          (bind (_direction _zitter) (`Timeline|Shake` :!via `PlayFromStart`)
            (:`Update`
              (`SceneComponent.K2_SetRelativeLocation` (`self.Platform`) (`KismetMathLibrary.MakeVector` 0.0 (* _zitter (`self.DirectionMovement`))) false false))
            (:`Finished`
              (`self.RestartTimeline`))))))
    (:`then_1`
      (`KismetSystemLibrary.Delay` 1.0)
      (`/Engine/EditorBlueprintResources/StandardMacros.DoOnce` false :!label _label_2
        (:`Completed`
          (bind (_direction_2 _fade1to0) (`Timeline|OpacityFadetoZero` :!via `PlayFromStart`)
            (:`Update`
              (`MaterialInstanceDynamic.SetScalarParameterValue` (`self.DynamicMaterial`) "Opacity" _fade1to0)
              (`KismetSystemLibrary.Delay` (`self.DisappearanceDuration`))
              (`SceneComponent.SetVisibility` (`self.Platform`) false false)
              (`PrimitiveComponent.SetCollisionEnabled` (`self.Platform_Collider`) "NoCollision"))
            (:`Finished`
              (goto _label_2 :!via `Reset`))))))))

(event `RestartTimeline`
  (goto _label :!via `Reset`))

(event `self.TriggerFade.OnComponentEndOverlap`
  (params (OverlappedComponent :type "PrimitiveComponent Object Reference") (OtherActor :type "Actor Object Reference") (OtherComp :type "PrimitiveComponent Object Reference") (OtherBodyIndex :type Integer))
  (`KismetSystemLibrary.Delay` 3.0)
  (`MaterialInstanceDynamic.SetScalarParameterValue` (`self.DynamicMaterial`) "Emissive" 0.0)
  (`/Engine/EditorBlueprintResources/StandardMacros.DoOnce` false :!label _label_3
    (:`Completed`
      (bind (_direction _opacitychange) (`Timeline|OpacityFadetoOne` :!via `PlayFromStart`)
        (:`Update`
          (`MaterialInstanceDynamic.SetScalarParameterValue` (`self.DynamicMaterial`) "Opacity" _opacitychange)
          (`SceneComponent.SetVisibility` (`self.Platform`) true false)
          (`PrimitiveComponent.SetCollisionEnabled` (`self.Platform_Collider`) "QueryAndPhysics")
          (goto _label_3 :!via `Reset`))))))

(fn `UserConstructionScript`)