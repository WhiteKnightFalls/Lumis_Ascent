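; BP_Collectable is a pickup actor that spins while idle and is collected once when BP_TPCharacter overlaps it.
; Collection plays a coin sound and a Timeline that moves, rotates and scales the Pivot and Niagara components, then destroys the actor on finish.
; The OnCollected event receives the character and here only prints a debug string.
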(event `self.ReceiveActorBeginOverlap`
  (params (OtherActor :type "Actor Object Reference"))
  ;[1 0.4219 0.6574] Animation wird abgespielt und aufgesammelt wenn triggered
  (bind _asbp_tpcharacter (cast `/Game/Blueprints/BP_Character/BP_TPCharacter` OtherActor))
  (`/Engine/EditorBlueprintResources/StandardMacros.DoOnce` false
    (:`Completed`
      (`self.PlayCollectAnimation`)
      (`self.OnCollected` _asbp_tpcharacter))))

(event `PlayCollectAnimation`
  ;[0.3833 0.8388 1] Collectanimation
  (`GameplayStatics.PlaySound2D` "/Game/Audio/SFX/coin-pickup-98269.coin-pickup-98269" 1.0 1.0 0.0 null null)
  (bind (_direction _z_movement _rotationspeed _size) (`Timeline|Timeline`)
    (:`Update`
      (`SceneComponent.K2_SetRelativeLocation` (`self.Pivot`) (* _z_movement (`self.Relative Location`)) false false)
      (`SceneComponent.K2_SetRelativeLocation` (`self.Niagara`) (* _z_movement (`self.Relative Location`)) false false)
      (`SceneComponent.K2_AddRelativeRotation` (`self.Pivot`) (`KismetMathLibrary.Conv_VectorToRotator` (* _rotationspeed (`self.Relative Rotation`))) false false)
      (`SceneComponent.K2_AddRelativeRotation` (`self.Niagara`) (`KismetMathLibrary.Conv_VectorToRotator` (* _rotationspeed (`self.Relative Rotation`))) false false)
      (`SceneComponent.SetWorldScale3D` (`self.Pivot`) (* _size (`self.Relative Size`)))
      (`SceneComponent.SetWorldScale3D` (`self.Niagara`) (* _size (`self.Relative Size`))))
    (:`Finished`
      (`self.K2_DestroyActor`))))

(event `OnCollected`
  (params (TPC :type "/Game/Blueprints/BP_Character/BP_TPCharacter Object Reference"))
  (`KismetSystemLibrary.PrintString` "Collected"))

(event `self.ReceiveTick`
  (params (DeltaSeconds :type "Float (single-precision)"))
  ;[0.2704 1 0.5268] Animation spint
  (`SceneComponent.K2_AddRelativeRotation` (`self.DefaultSceneRoot`) (`KismetMathLibrary.MakeRotator` 0.0 0.0 (* (`self.IdleRotSpeed`) (`GameplayStatics.GetWorldDeltaSeconds`))) false false))

(fn `UserConstructionScript`)