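; BP_BouncingPlatform is a bounce pad that launches BP_TPCharacter upward when the character lands on it.
; Tick spins the OuterRing and BouncingStar components at separate idle yaw speeds, scaled by delta time.
; Any hit plays a 2D sound, while a hit normal Z check limits the launch to contacts from above.
; After a launch, a timeline restarts to drive extra spin on both components.
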(event `self.ReceiveTick`
  (params (DeltaSeconds :type "Float (single-precision)"))
  (`SceneComponent.K2_AddRelativeRotation` (`self.OuterRing`) (`KismetMathLibrary.MakeRotator` 0.0 0.0 (* (`self.IdleRotSpeedOuterRing`) (`GameplayStatics.GetWorldDeltaSeconds`))) false false)
  (`SceneComponent.K2_AddRelativeRotation` (`self.BouncingStar`) (`KismetMathLibrary.MakeRotator` 0.0 0.0 (* (`self.IdleRotSpeedStar`) (`GameplayStatics.GetWorldDeltaSeconds`))) false false))

(event `self.ReceiveHit`
  (params (MyComp :type "PrimitiveComponent Object Reference") (Other :type "Actor Object Reference") (OtherComp :type "PrimitiveComponent Object Reference") (bSelfMoved :type Boolean) (HitLocation :type "Vector Structure") (HitNormal :type "Vector Structure") (NormalImpulse :type "Vector Structure") (Hit :type "HitResult Structure (by ref)"))
  (`GameplayStatics.PlaySound2D` "/Game/Audio/SFX/BouncyPlatform.BouncyPlatform" 1.0 1.0 0.0 null null)
  (if (<= (.z HitNormal) -0.5)
    (bind _asbp_tpcharacter (cast `/Game/Blueprints/BP_Character/BP_TPCharacter` Other))
    (`Character.LaunchCharacter` _asbp_tpcharacter (`KismetMathLibrary.MakeVector` 0.0 0.0 (`self.Launch Strenght`)) false false)
    (bind (_direction _rotationspeed) (`Timeline|Timeline` :!via `PlayFromStart`)
      (:`Update`
        (`SceneComponent.K2_AddRelativeRotation` (`self.BouncingStar`) (`KismetMathLibrary.MakeRotator` 0.0 0.0 (* _rotationspeed (`self.relativeRotation`) (`GameplayStatics.GetWorldDeltaSeconds`))) false false)
        (`SceneComponent.K2_AddRelativeRotation` (`self.OuterRing`) (`KismetMathLibrary.MakeRotator` 0.0 0.0 (* _rotationspeed (`self.relativeRotation`) (`GameplayStatics.GetWorldDeltaSeconds`))) false false))
      (:`Finished`
        (`/Engine/EditorBlueprintResources/StandardMacros.DoOnce` false :!via `Reset`)))))

(fn `UserConstructionScript`)