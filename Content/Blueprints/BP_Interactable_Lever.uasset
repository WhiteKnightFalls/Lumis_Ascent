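; BP_Interactable_Lever is an interactable lever that starts a linked moving platform when used.
; Interact calls its parent, then passes a DoOnce to play a timeline that pitches the Pivot up to 60 degrees.
; Timeline updates also call the platform's StartonInteractedLever through a short Delay, so that call can repeat during playback.
; When the timeline finishes, ResetInteraction resets the DoOnce so the lever can be used again.
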(event `self.Interact`
  (`parent.Interact`)
  (`/Engine/EditorBlueprintResources/StandardMacros.DoOnce` false :!label _label
    (:`Completed`
      (bind (_direction _activate) (`Timeline|Timeline` :!via `PlayFromStart`)
        (:`Update`
          (`SceneComponent.K2_SetRelativeRotation` (`self.Pivot`) (`KismetMathLibrary.MakeRotator` 0.0 (* _activate 60.0)) false false)
          (`KismetSystemLibrary.Delay` 0.2)
          (`/Game/Blueprints/BP_InteractableLever_MovingPlatform.StartonInteractedLever` (`self.MovingPlatformLtoR`)))
        (:`Finished`
          (`self.ResetInteraction`))))))

(event `ResetInteraction`
  (goto _label :!via `Reset`))

(fn `UserConstructionScript`
  (`parent.UserConstructionScript`))