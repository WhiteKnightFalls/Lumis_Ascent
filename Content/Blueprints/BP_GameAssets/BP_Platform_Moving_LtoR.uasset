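; A moving platform that shuttles back and forth along DirectionMovement, starting automatically at BeginPlay after an initial delay.
; A timeline's MoveToPos track, multiplied by DirectionMovement, sets the Platform component's relative location without sweep.
; A FlipFlop alternates playing and reversing the timeline with its own delay before each leg, and the timeline's Finished pin re-enters it to loop endlessly.
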(event `self.ReceiveBeginPlay`
  (`KismetSystemLibrary.Delay` (`self.DelayFirst`))
  (`/Engine/EditorBlueprintResources/StandardMacros.FlipFlop` :!label _label
    (:`A`
      (`KismetSystemLibrary.Delay` (`self.DelayEnd`))
      (bind (_direction _movetopos) (`Timeline|Timeline` :!label _label_2)
        (:`Update`
          (`SceneComponent.K2_SetRelativeLocation` (`self.Platform`) (* _movetopos (`self.DirectionMovement`)) false false))
        (:`Finished`
          (goto _label))))
    (:`B`
      (`KismetSystemLibrary.Delay` (`self.DelayStart`))
      (goto _label_2 :!via `Reverse`))))

(fn `UserConstructionScript`)