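; BP_Collectable is a spinning pickup that a BP_TPCharacter collects once by overlapping it.
; Tick yaws the root at IdleRotSpeed, scaled by delta time.
; On collection, a timeline moves, rotates and scales Pivot, then destroys the actor, while OnCollected only prints a message.
; Pivot's scale multiplies the Size track by RelativeRotation, leaving RelativeSize unused.
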(event `self.ReceiveActorBeginOverlap`
  (params (OtherActor :type "Actor Object Reference"))
  (cast `/Game/Blueprints/BP_TPCharacter` OtherActor)
  (`/Engine/EditorBlueprintResources/StandardMacros.DoOnce` false
    (:`Completed`
      (`self.PlayCollectAnimation`)
      (`self.OnCollected`))))

(event `PlayCollectAnimation`
  (bind (_direction _z_movement _rotationspeed _size) (`Timeline|Timeline`)
    (:`Update`
      (`SceneComponent.K2_SetRelativeLocation` (`self.Pivot`) (* _z_movement (`self.Relative Location`)) false false)
      (`SceneComponent.K2_AddRelativeRotation` (`self.Pivot`) (`KismetMathLibrary.Conv_VectorToRotator` (* _rotationspeed (`self.Relative Rotation`))) false false)
      (`SceneComponent.SetWorldScale3D` (`self.Pivot`) (* _size (`self.Relative Rotation`))))
    (:`Finished`
      (`self.K2_DestroyActor`))))

(event `OnCollected`
  (`KismetSystemLibrary.PrintString` "Collected"))

(event `self.ReceiveTick`
  (params (DeltaSeconds :type "Float (single-precision)"))
  (`SceneComponent.K2_AddRelativeRotation` (`self.DefaultSceneRoot`) (`KismetMathLibrary.MakeRotator` 0.0 0.0 (* (`self.IdleRotSpeed`) (`GameplayStatics.GetWorldDeltaSeconds`))) false false))

(fn `UserConstructionScript`)